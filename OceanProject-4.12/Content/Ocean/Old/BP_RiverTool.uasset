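; BP_RiverTool is a construction-time spline tool that lays a surface mesh along a path, named for building rivers.
; The construction script splits the spline length by Spacing and adds a collidable spline mesh per segment, with the set mesh, material and Width.
; Segments use manual attachment, so their endpoints come from world-space spline locations, with tangents from spline direction scaled by TangentScale.
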(fn `UserConstructionScript`
  (bind _splinecomponent (`self.SplineComponent`))
  (bind _spacing (`self.Spacing`))
  (bind _tangentscale (`self.TangentScale`))
  ;[1 1 1] SplineTool Construction
  (for _index (range (+ (`.ReturnValue` (`KismetMathLibrary.FMod` (`SplineComponent.GetSplineLength` _splinecomponent) _spacing)) 1))
    (bind _returnvalue (`AddComponent|SplineMeshComponent_37` :`bManualAttachment` true)) ; Add the index value SplineComponent to the Pline
    (`PrimitiveComponent.SetCollisionEnabled` _returnvalue "QueryAndPhysics") ; Set Collision for the Road mesh
    (`StaticMeshComponent.SetStaticMesh` _returnvalue (`self.SurfaceMesh`))
    (`PrimitiveComponent.SetMaterial` _returnvalue 0 (`self.SurfaceMaterial`))
    (`SplineMeshComponent.SetStartScale` _returnvalue (`KismetMathLibrary.MakeVector2D` 1.0 (`self.Width`)) true)
    (`SplineMeshComponent.SetEndScale` _returnvalue (`KismetMathLibrary.MakeVector2D` 1.0 (`self.Width`)) true)
    (bind _returnvalue_2 (* _index _spacing))
    (bind _returnvalue_3 (+ _returnvalue_2 _spacing))
    (`SplineMeshComponent.SetStartAndEnd` _returnvalue (`SplineComponent.GetWorldLocationAtDistanceAlongSpline` _splinecomponent _returnvalue_2) (* (`SplineComponent.GetWorldDirectionAtDistanceAlongSpline` _splinecomponent _returnvalue_2) _tangentscale) (`SplineComponent.GetWorldLocationAtDistanceAlongSpline` _splinecomponent _returnvalue_3) (* (`SplineComponent.GetWorldDirectionAtDistanceAlongSpline` _splinecomponent _returnvalue_3) _tangentscale) true)))